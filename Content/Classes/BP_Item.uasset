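; BP_Item is an item actor with a type of weapon, tool or consumable, plus empty Pickup, Drop and Use events.
; On BeginPlay, Constructor gives weapons random damage and a shuffled name, zeroing damage for other types.
; It prints these, then after a delay looks up a BP_Enemy and calls Attack, which subtracts scaled damage from enemy health.
; A timeline also drives the Sphere's relative height.
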(event Custom|Pick%20up)

(event Custom|Drop)

(event Custom|Use)

(event EventBeginPlay
  (Utilities|FlowControl|Sequence
    (:then_0
      (CallFunction|Constructor)
      (Development|PrintString (Utilities|String|Append "Name:" (Variables|Default|GetName) (Utilities|String|ToString(Integer) (Variables|Default|GetDamage))))
      (Utilities|FlowControl|Delay 5.0)
      (Actor|GetActorOfClass "/Game/Blueprints/BP_Enemy.BP_Enemy_C")
      (CallFunction|Attack))
    (:then_1
      (bind _newtrack_0 (Timeline|Timeline Play)
        (:Update
          (Transformation|SetRelativeLocation (Variables|Default|GetSphere) (Math|Vector|MakeVector 0.0 0.0 (Math|Float|Lerp 0.0 1e+02 _newtrack_0)) false false))))))

(fn ConstructionScript)

(fn Constructor
  (bind _weaponnames (Variables|Default|GetWeaponNames))
  (switch Utilities|FlowControl|Switch|SwitchonEItemType (Variables|Default|GetType)
    (:NewEnumerator0
      (Variables|Default|SetDamage (Math|Random|RandomIntegerinRange 3 6))
      (if true ; if true, randomize name
        (Utilities|Array|Shuffle _weaponnames)
        (Variables|Default|SetName (Utilities|Array|Get(acopy) _weaponnames))))
    (:NewEnumerator1
      (Variables|Default|SetDamage 0))
    (:NewEnumerator2
      (Variables|Default|SetDamage 0))))

(fn Attack
  (params (GivenEnemy :type BP%20Enemy%20Object%20Reference))
  (Variables|/Game/Blueprints/BP_Enemy.BP_Enemy_C|SetHealth GivenEnemy (- (Variables|/Game/Blueprints/BP_Enemy.BP_Enemy_C|GetHealth GivenEnemy) (* (Math|Conversions|ToFloat(Integer) (Variables|Default|GetDamage)) 0.01))))